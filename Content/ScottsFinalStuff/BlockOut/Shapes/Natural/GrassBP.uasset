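; GrassBP is a grass prop Blueprint that varies its look per instance, with all work done in the Construction Script.
; Optional toggles randomise each scale axis independently within a shared range and give the mesh a random yaw.
; A dynamic instance of Grass_Inst receives either a random red-green Colour or the set Colour variable.
; The randomness is unseeded, so values reroll whenever construction reruns, and the event graph is inactive.
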(event EventBeginPlay
  (|CallParentFunction))

(event Collision|EventActorBeginOverlap
  (params (OtherActor :type Actor%20Object%20Reference))
  (|CallParentFunction OtherActor))

(event EventTick
  (params (DeltaSeconds :type Float%20%28single-precision%29))
  (|CallParentFunction DeltaSeconds))

(fn ConstructionScript
  (bind _max_size_0 (Variables|Transform|GetMax_Size_0))
  (bind _min_size_0 (Variables|Transform|GetMin_Size_0))
  (bind _returnvalue (Math|Random|RandomFloatinRange _min_size_0 _max_size_0))
  (if (Variables|Default|GetRandomise%20Size)
    (Transformation|SetActorScale3D (Math|Vector|MakeVector _returnvalue _returnvalue _returnvalue)))
  (if (Variables|Grass|GetRandom_Rotation?)
    (Transformation|SetRelativeRotation (Variables|Character|GetMesh) (Math|Rotator|MakeRotator 0.0 0.0 (Math|Random|RandomFloatinRange 0.0 3.6e+02)) false false))
  (bind _returnvalue_2 (Rendering|Material|CreateDynamicMaterialInstance (Variables|Character|GetMesh) 0 "/Game/ScottsFinalStuff/BlockOut/Materials_Textures/Grass_Inst.Grass_Inst" "None" :!class /Script/Engine.PrimitiveComponent))
  (if (Variables|Grass|GetRandom_Colour?)
    (Rendering|Material|SetVectorParameterValue _returnvalue_2 "Colour" (Utilities|Struct|MakeLinearColor (Math|Random|RandomFloatinRange 0.0 (Variables|Grass|GetMax_Red)) (Math|Random|RandomFloatinRange 0.1 (Variables|Grass|GetMax_Green)) 0.0 1.0) :!class /Script/Engine.MaterialInstanceDynamic)
    (else
      (Rendering|Material|SetVectorParameterValue _returnvalue_2 "Colour" (Variables|Grass|GetColour) :!class /Script/Engine.MaterialInstanceDynamic))))